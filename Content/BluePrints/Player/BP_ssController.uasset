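; BP_ssController is a player controller Blueprint that provides debug input for testing the inventory with consumable potions.
; One debug key adds a potion through the InventoryComponent and the other uses one, each identified by gameplay tag.
; Each key has its own FlipFlop, so successive presses alternate between health and mana potions independently of the other key.
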(event Input|KeyboardEvents|DebugKey1
  (params (Key :type Key%20Structure :default "None") (ActionValue :type Input%20Action%20Value%20Structure))
  (:Pressed
    (Utilities|FlowControl|FlipFlop
      (:A
        (Class|SsInventoryComponent|AddItem (Variables|Default|GetInventoryComponent) (GameplayTags|MakeLiteralGameplayTag "(TagName=\"Item.Consumable.HealthPotion\")") 1))
      (:B
        (Class|SsInventoryComponent|AddItem (Variables|Default|GetInventoryComponent) (GameplayTags|MakeLiteralGameplayTag "(TagName=\"Item.Consumable.ManaPotion\")") 1)))))

(event Input|KeyboardEvents|DebugKey2
  (params (Key :type Key%20Structure :default "None") (ActionValue :type Input%20Action%20Value%20Structure))
  (:Pressed
    (Utilities|FlowControl|FlipFlop
      (:A
        (Class|SsInventoryComponent|UseItem (Variables|Default|GetInventoryComponent) (GameplayTags|MakeLiteralGameplayTag "(TagName=\"Item.Consumable.HealthPotion\")") 1))
      (:B
        (Class|SsInventoryComponent|UseItem (Variables|Default|GetInventoryComponent) (GameplayTags|MakeLiteralGameplayTag "(TagName=\"Item.Consumable.ManaPotion\")") 1)))))

(fn ConstructionScript)